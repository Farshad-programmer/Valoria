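; Overview demo actor that animates a tagged sphere map border and shows its point-inside-area check on helper actors.
; On BeginPlay it caches the first tagged BP_Sphere_Border and all tagged BP_Helper actors.
; Each Tick it pulses the sphere size along a sine of accumulated time, updates the border at runtime, then sets each helper's active state by whether its location lies inside.
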(event EventBeginPlay
  (bind _outactors (Actor|GetAllActorsOfClasswithTag "/Game/Assets/MapBorderCollection/Blueprints/BP_Sphere_Border.BP_Sphere_Border_C" "SphereBorder"))
  (Variables|Default|SetSphereBorder (Utilities|Array|Get(acopy) _outactors))
  (bind _outactors_2 (Actor|GetAllActorsOfClasswithTag "/Game/Assets/MapBorderCollection/Overview/Blueprints/Helper/BP_Helper.BP_Helper_C" "SphereHelper"))
  (Variables|Default|SetHelpers _outactors_2))

(event EventTick
  (params (DeltaSeconds :type Float%20%28single-precision%29))
  (Utilities|IsValid (Variables|Default|GetSphereBorder)
    (:Is%20Valid
      (Variables|Default|SetDeltaTIme DeltaSeconds)
      (Variables|Default|SetTime (+ (Variables|Default|GetDeltaTIme) (Variables|Default|GetTime)))
      (Utilities|FlowControl|Sequence
        (:then_0
          (Variables|/Game/Assets/MapBorderCollection/Blueprints/BP_Sphere_Border.BP_Sphere_Border_C|SetSphereSize (Variables|Default|GetSphereBorder) (+ (* (Math|Trig|Sin(Radians) (Variables|Default|GetTime)) 2e+03) 2e+03))
          (Default|UpdateBorderinRuntime (Variables|Default|GetSphereBorder) false))
        (:then_1
          (for _array_element (Variables|Default|GetHelpers)
            (bind _success (Default|CheckifPointLiesInsideArea (Variables|Default|GetSphereBorder) (Transformation|GetActorLocation _array_element)))
            (Default|SetNewActiveState _array_element _success)))))))

(fn ConstructionScript)