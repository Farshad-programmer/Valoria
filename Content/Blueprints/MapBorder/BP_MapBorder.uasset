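; BP_MapBorder is a map territory border that reflects its ownership status: self, ownerless, ally or enemy.
; After a short BeginPlay delay it caches its child decal actor, and UpdateBorders recolors that decal by status, also via UpdateBorderOwner.
; Tick disables the border box's collision only for self-owned borders.
; An overlap box links city centers back to this border and prints a debug flag; clearing that link on exit is unwired.
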(event OnComponentBeginOverlap(cityCenterboxChecker)
  (params (OverlappedComponent :type Primitive%20Component%20Object%20Reference) (OtherActor :type Actor%20Object%20Reference) (OtherComp :type Primitive%20Component%20Object%20Reference) (OtherBodyIndex :type Integer) (bFromSweep :type Boolean) (SweepResult :type Hit%20Result%20Structure%20%28by%20ref%29))
  (bind _asbp_city_center (Utilities|Casting|CastToBP_CityCenter OtherActor))
  (Variables|Default|SetAs%20BP%20City%20Center _asbp_city_center)
  (bind _output_get (Variables|/Script/Valoria.Building|SetBorderRef _asbp_city_center self))
  (Development|PrintString (Utilities|String|ToString(Boolean) (Variables|/Script/Valoria.MapBorder|GetbBorderHasCityCenter _output_get))))

(event OnComponentEndOverlap(cityCenterboxChecker)
  (params (OverlappedComponent :type Primitive%20Component%20Object%20Reference) (OtherActor :type Actor%20Object%20Reference) (OtherComp :type Primitive%20Component%20Object%20Reference) (OtherBodyIndex :type Integer))
  (bind _asbp_city_center (Utilities|Casting|CastToBP_CityCenter OtherActor)))

(event EventBeginPlay
  (Utilities|FlowControl|Delay 0.2)
  (bind _asbp_decal_border (Utilities|Casting|CastToBP_Decal_Border (Variables|/Script/Engine.ChildActorComponent|GetChildActor (Variables|Default|GetChildActor))))
  (Variables|Default|SetAs%20BP%20Decal%20Border _asbp_decal_border)
  (CallFunction|UpdateBorders (Variables|Default|GetborderStatus)))

(event EventUpdateBorderOwner
  (params (status :type EBorderStatus%20Enum :default "self"))
  ;[1 1 1] Will be expanded later
  (CallFunction|UpdateBorders status))

(event EventTick
  (params (DeltaSeconds :type Float%20%28single-precision%29))
  (Utilities|FlowControl|Sequence
    (:then_0
      (if (Utilities|Enum|Equal(Enum) (Variables|Default|GetborderStatus) "self")
        (Collision|SetCollisionEnabled (Variables|Default|Getborderbox) "NoCollision")
        (else
          (Collision|SetCollisionEnabled (Variables|Default|Getborderbox) "QueryAndPhysics"))))))

(fn ConstructionScript)

(fn UpdateBorders
  (params (Selection :type EBorderStatus%20Enum :default "self"))
  (bind _as_bp_decal_border (Variables|Default|GetAs%20BP%20Decal%20Border))
  (switch Utilities|FlowControl|Switch|SwitchonEBorderStatus Selection
    (:self
      (Variables|/Game/Assets/MapBorderCollection/Blueprints/BP_Decal_Border.BP_Decal_Border_C|SetBorderColor _as_bp_decal_border "(R=0.000000,G=20.000000,B=2.500000,A=1.000000)"))
    (:ownerless
      (Variables|/Game/Assets/MapBorderCollection/Blueprints/BP_Decal_Border.BP_Decal_Border_C|SetBorderColor _as_bp_decal_border "(R=0.024399,G=0.026042,B=0.000000,A=1.000000)"))
    (:ally
      (Variables|/Game/Assets/MapBorderCollection/Blueprints/BP_Decal_Border.BP_Decal_Border_C|SetBorderColor _as_bp_decal_border "(R=20.000000,G=13.756205,B=0.000000,A=1.000000)"))
    (:enemy
      (Variables|/Game/Assets/MapBorderCollection/Blueprints/BP_Decal_Border.BP_Decal_Border_C|SetBorderColor _as_bp_decal_border "(R=20.000000,G=0.000000,B=0.640000,A=1.000000)")))
  (Default|UpdateBorderinRuntime (Variables|Default|GetAs%20BP%20Decal%20Border)))