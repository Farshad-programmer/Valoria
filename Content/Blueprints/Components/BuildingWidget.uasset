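; Actor component that keeps a Building's worker widget in sync with that building's state.
; BeginPlay caches the owning Building and its WBP_BuildingWorker widget, then seeds the worker count and construction progress values.
; Tick refreshes those values every frame, hides the worker text when the count is zero, and shows the widget component only while the player pawn is within a set distance.
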(event EventBeginPlay
  (bind _asbuilding (Utilities|Casting|CastToBuilding (Components|GetOwner)))
  (Variables|Default|SetAs%20Building _asbuilding)
  (bind _aswbp_building_worker (Utilities|Casting|CastToWBP_BuildingWorker (UserInterface|GetWidget (Variables|/Script/Valoria.Building|GetWidget _asbuilding))))
  (Variables|Default|SetAs%20WBP%20Building%20Worker _aswbp_building_worker)
  (Rendering|Components|TextRender|SetText (Variables|/Game/Blueprints/HUD/Widget/WBP_BuildingWorker.WBP_BuildingWorker_C|GetTB_Worker _aswbp_building_worker) (Utilities|Text|ToText(Integer) (Variables|/Script/Valoria.Building|GetworkerNumber _asbuilding)))
  (Variables|/Game/Blueprints/HUD/Widget/WBP_BuildingWorker.WBP_BuildingWorker_C|SetConstructionCurrentValue _aswbp_building_worker (Variables|/Script/Valoria.Building|GetconstructionCounter _asbuilding))
  (Variables|/Game/Blueprints/HUD/Widget/WBP_BuildingWorker.WBP_BuildingWorker_C|SetConstructionFinishValue _aswbp_building_worker (Variables|/Script/Valoria.Building|GetconstrcutionFinishValue _asbuilding)))

(event EventTick
  (params (DeltaSeconds :type Float%20%28single-precision%29))
  (bind _as_building (Variables|Default|GetAs%20Building))
  (bind _as_building_2 (Variables|Default|GetAs%20Building))
  (bind _as_wbp_building_worker (Variables|Default|GetAs%20WBP%20Building%20Worker))
  (bind _workernumber (Variables|/Script/Valoria.Building|GetworkerNumber _as_building_2))
  (bind _tb_worker (Variables|/Game/Blueprints/HUD/Widget/WBP_BuildingWorker.WBP_BuildingWorker_C|GetTB_Worker _as_wbp_building_worker))
  (Utilities|IsValid _as_building_2
    (:Is%20Valid
      (Utilities|IsValid _as_wbp_building_worker
        (:Is%20Valid
          (Utilities|FlowControl|Sequence
            (:then_0
              (Rendering|Components|TextRender|SetText _tb_worker (Utilities|Text|ToText(Integer) _workernumber))
              (Variables|/Game/Blueprints/HUD/Widget/WBP_BuildingWorker.WBP_BuildingWorker_C|SetConstructionCurrentValue _as_wbp_building_worker (Variables|/Script/Valoria.Building|GetconstructionCounter _as_building))
              (Variables|/Game/Blueprints/HUD/Widget/WBP_BuildingWorker.WBP_BuildingWorker_C|SetConstructionFinishValue _as_wbp_building_worker (Variables|/Script/Valoria.Building|GetconstrcutionFinishValue _as_building))
              (if (== _workernumber 0)
                (Widget|SetVisibility _tb_worker "Hidden")
                (else
                  (Widget|SetVisibility _tb_worker "Visible"))))
            (:then_1
              (Rendering|SetVisibility (Variables|/Script/Valoria.Building|GetWidget (Variables|Default|GetAs%20Building)) (<= (Transformation|GetDistanceTo (Game|Player|GetPlayerPawn 0) (Variables|Default|GetAs%20Building)) 4e+03) false))))))))