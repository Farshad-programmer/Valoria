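; Component that keeps the floating widget on a ResourceMaster actor in sync with that resource's state.
; BeginPlay caches the owner and its WBP_ResourseWorker widget, then fills in worker count and current and finish resource values.
; Tick re-pushes those values every frame, hides the worker text when no workers are assigned, and shows the whole widget only while the player pawn is within a set distance.
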(event EventBeginPlay
  (bind _asresource_master (Utilities|Casting|CastToResourceMaster (Components|GetOwner)))
  (bind _output_get (Variables|Default|SetAs%20Resource%20Master _asresource_master))
  (bind _aswbp_resourse_worker (Utilities|Casting|CastToWBP_ResourseWorker (UserInterface|GetWidget (Variables|/Script/Valoria.ResourceMaster|GetWidget _asresource_master))))
  (bind _output_get_2 (Variables|Default|SetAs%20WBP%20Resourse%20Worker _aswbp_resourse_worker))
  (Rendering|Components|TextRender|SetText (Variables|/Game/Blueprints/HUD/Widget/WBP_ResourseWorker.WBP_ResourseWorker_C|GetTB_Worker _output_get_2) (Utilities|Text|ToText(Integer) (Variables|/Script/Valoria.ResourceMaster|GetworkerNumber _output_get)))
  (Variables|/Game/Blueprints/HUD/Widget/WBP_ResourseWorker.WBP_ResourseWorker_C|SetResourseCurrentValue _output_get_2 (Variables|/Script/Valoria.ResourceMaster|GetresourceCounter (Variables|Default|GetAs%20Resource%20Master)))
  (Variables|/Game/Blueprints/HUD/Widget/WBP_ResourseWorker.WBP_ResourseWorker_C|SetResourseFinishValue _output_get_2 (Variables|/Script/Valoria.ResourceMaster|GetresourceFinishValue (Variables|Default|GetAs%20Resource%20Master))))

(event EventTick
  (params (DeltaSeconds :type Float%20%28single-precision%29))
  (bind _as_resource_master (Variables|Default|GetAs%20Resource%20Master))
  (bind _as_resource_master_2 (Variables|Default|GetAs%20Resource%20Master))
  (bind _as_wbp_resourse_worker (Variables|Default|GetAs%20WBP%20Resourse%20Worker))
  (bind _workernumber (Variables|/Script/Valoria.ResourceMaster|GetworkerNumber _as_resource_master_2))
  (bind _tb_worker (Variables|/Game/Blueprints/HUD/Widget/WBP_ResourseWorker.WBP_ResourseWorker_C|GetTB_Worker _as_wbp_resourse_worker))
  (Utilities|IsValid _as_resource_master_2
    (:Is%20Valid
      (Utilities|IsValid _as_wbp_resourse_worker
        (:Is%20Valid
          (Utilities|FlowControl|Sequence
            (:then_0
              (Rendering|Components|TextRender|SetText _tb_worker (Utilities|Text|ToText(Integer) _workernumber))
              (Variables|/Game/Blueprints/HUD/Widget/WBP_ResourseWorker.WBP_ResourseWorker_C|SetResourseCurrentValue _as_wbp_resourse_worker (Variables|/Script/Valoria.ResourceMaster|GetresourceCounter _as_resource_master))
              (Variables|/Game/Blueprints/HUD/Widget/WBP_ResourseWorker.WBP_ResourseWorker_C|SetResourseFinishValue _as_wbp_resourse_worker (Variables|/Script/Valoria.ResourceMaster|GetresourceFinishValue _as_resource_master))
              (if (== _workernumber 0)
                (Widget|SetVisibility _tb_worker "Hidden")
                (else
                  (Widget|SetVisibility _tb_worker "Visible"))))
            (:then_1
              (Rendering|SetVisibility (Variables|/Script/Valoria.ResourceMaster|GetWidget (Variables|Default|GetAs%20Resource%20Master)) (<= (Transformation|GetDistanceTo (Game|Player|GetPlayerPawn 0) (Variables|Default|GetAs%20Resource%20Master)) 4e+03) false))))))))