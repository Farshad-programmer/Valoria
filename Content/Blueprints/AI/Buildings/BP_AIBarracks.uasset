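; AI barracks building Blueprint that drives the construction panel of the game's base HUD.
; On BeginPlay it creates its own WBP_Base widget linked to the player's BP_ValoriaCam pawn, adds it to the viewport and sets Game and UI input.
; ConstructionHUD shows or collapses the construction widget switcher, selecting the page by index and registering this barracks with the widget; its Building input is unused.
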(event EventBeginPlay
  (bind _asbp_valoria_cam (Utilities|Casting|CastToBP_ValoriaCam (Game|Player|GetPlayerPawn 0)))
  (bind _returnvalue (UserInterface|CreateWidget "/Game/Blueprints/HUD/Widget/WBP_Base.WBP_Base_C" 0 _asbp_valoria_cam))
  (bind _output_get (Variables|Default|SetGameBaseWidgetRef _returnvalue))
  (UserInterface|Viewport|AddtoViewport _output_get 0)
  (Input|SetInputModeGameandUI (Game|GetPlayerController 0) 0 "DoNotLock" true false))

(event EventConstructionHUD
  (params (active :type Boolean) (constructNum :type Integer) (building :type Building%20Object%20Reference))
  (bind _gamebasewidgetref (Variables|Default|GetGameBaseWidgetRef))
  (bind _widgetswitcher_construction (Variables|/Game/Blueprints/HUD/Widget/WBP_Base.WBP_Base_C|GetWidgetSwitcher_Construction _gamebasewidgetref))
  (if active
    (Utilities|IsValid _gamebasewidgetref
      (:Is%20Valid
        (Widget|SetVisibility _widgetswitcher_construction "Visible")
        (Variables|/Script/UMG.WidgetSwitcher|SetActiveWidgetIndex _widgetswitcher_construction constructNum)
        (Variables|/Game/Blueprints/HUD/Widget/WBP_Base.WBP_Base_C|SetBarracksRef _gamebasewidgetref self)))
    (else
      (Utilities|IsValid _gamebasewidgetref
        (:Is%20Valid
          (Widget|SetVisibility _widgetswitcher_construction "Collapsed"))))))

(fn ConstructionScript)