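; BP_ValoriaAI holds a non-player capital's diplomatic status (Ally, Neutral or Enemy) and propagates it to units and the map border.
; UpdateAIStatus-NonPlayer scans every ValoriaCharacter, gives same-capital units that status and appends code 1 to their attack list.
; Player-tagged units of other capitals always become Enemy, a noted stopgap that should apply only toward enemy capitals.
; It then copies the status to the referenced border and refreshes it.
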(event Custom|UpdateAIStatus-NonPlayer
  (bind _mapborderref (Variables|Default|GetmapBorderRef))
  (Utilities|FlowControl|Sequence
    (:then_0
      (bind _outactors (Actor|GetAllActorsOfClass "/Script/Valoria.ValoriaCharacter"))
      (for _array_element _outactors
        ;[1 1 1] Change AI team to become Enemy for the player
        (if (== (Variables|/Script/Valoria.ValoriaCharacter|GetcapitalCode _array_element) (Variables|Default|GetcapitalCode))
          (Variables|/Script/Valoria.ValoriaCharacter|SetenemyStatus _array_element (Variables|Default|GetenemyStatus))
          (Utilities|Array|Add (Variables|/Script/Valoria.ValoriaCharacter|GetenemyUnitCodeToAttack _array_element) 1)
          (else
            ;[1 1 1] Make Player soldiers enemy status = enemy -  but it must later be fixed because the player need to only become enemy for enemy capitals!
            (if (Actor|ActorHasTag _array_element "Player")
              (Variables|/Script/Valoria.ValoriaCharacter|SetenemyStatus _array_element "enemy"))))))
    (:then_1
      (switch Utilities|FlowControl|Switch|SwitchonEAIStatus (Variables|Default|GetenemyStatus)
        (:ally
          (Variables|/Script/Valoria.MapBorder|SetborderStatus _mapborderref "ally"))
        (:neutral
          (Variables|/Script/Valoria.MapBorder|SetborderStatus _mapborderref "neutral"))
        (:enemy
          (Variables|/Script/Valoria.MapBorder|SetborderStatus _mapborderref "enemy")))
      (Class|MapBorder|UpdateBorderOwnerfromBlueprint _mapborderref))))

(fn ConstructionScript)