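; BP_ValoriaWorker is a worker character Blueprint that shows its health through an overlay widget.
; BeginPlay caches the Widget component's WBP_CharacterOverlay, and Tick copies Health and MaxHealth into it every frame while that reference is valid.
; An unconnected branch would make the capsule ignore the Visibility channel for actors tagged Player, but it never runs.
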(event EventBeginPlay
  (bind _aswbp_character_overlay (Utilities|Casting|CastToWBP_CharacterOverlay (UserInterface|GetWidget (Variables|Default|GetWidget))))
  (Variables|Default|SetWBPCharacterOverlayRef _aswbp_character_overlay))

(event EventTick
  (params (DeltaSeconds :type Float%20%28single-precision%29))
  (bind _wbpcharacteroverlayref (Variables|Default|GetWBPCharacterOverlayRef))
  (Utilities|FlowControl|Sequence
    (:then_0
      (Utilities|IsValid _wbpcharacteroverlayref
        (:Is%20Valid
          (Variables|/Game/Blueprints/HUD/Widget/WBP_CharacterOverlay.WBP_CharacterOverlay_C|SetHealth _wbpcharacteroverlayref (Variables|Default|Gethealth))
          (Variables|/Game/Blueprints/HUD/Widget/WBP_CharacterOverlay.WBP_CharacterOverlay_C|SetMaxHealth _wbpcharacteroverlayref (Variables|Default|GetmaxHealth)))))))

(fn ConstructionScript)